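; BP_FollowCamera is an actor that follows the side-scroller player character at a fixed Offset.
; BeginPlay casts player 0's character to BP_SideScrollerCharacter and caches it.
; Tick snaps the actor to that character's location plus Offset, with no smoothing or sweep.
; The construction script applies the same placement to the first BP_SideScrollerCharacter it finds, so the actor lines up before play.
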(event `self.ReceiveBeginPlay`
  ;[0 0 0 0.5] Stores a reference to the player
  (bind _asbp_side_scroller_character (cast `/Game/Blueprints/BP_SideScrollerCharacter` (`GameplayStatics.GetPlayerCharacter` 0)))
  (set `self.PlayerReference` _asbp_side_scroller_character))

(event `self.ReceiveTick`
  (params (DeltaSeconds :type "Float (single-precision)"))
  ;[0 0 0 0.5] Prevents the player from going off the platform
  (`self.K2_SetActorLocation` (+ (`self.K2_GetActorLocation` (`self.PlayerReference`)) (`self.Offset`))))

(fn `UserConstructionScript`
  ;[0 0 0 0.5] Player stays on platform
  (bind _returnvalue (`GameplayStatics.GetActorOfClass` "/Game/Blueprints/BP_SideScrollerCharacter.BP_SideScrollerCharacter_C"))
  (`self.K2_SetActorLocation` (+ (`self.K2_GetActorLocation` _returnvalue) (`self.Offset`))))